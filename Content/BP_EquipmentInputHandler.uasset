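; BP_EquipmentInputHandler is an actor that lets the player select arm equipment slots through input actions.
; On BeginPlay it enables input from the first player controller.
; Six Enhanced Input actions each cast the first player character to FGCharacterPlayer and call SelectArmEquipmentByIndex with the matching zero-based slot index.
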(event `EnhancedInput|/EquipmentKeyBindings/Inputs/Player/Actions/IA_TriggerSelectEquipment_04`
  (params (ActionValue :type Boolean) (ElapsedSeconds :type "Float (double-precision)") (TriggeredSeconds :type "Float (double-precision)") (InputAction :type "InputAction Object Reference" :default "/EquipmentKeyBindings/Inputs/Player/Actions/IA_TriggerSelectEquipment_04.IA_TriggerSelectEquipment_04"))
  (:`Triggered`
    (bind _asfgcharacter_player (cast `FGCharacterPlayer` (`GameplayStatics.GetPlayerCharacter` 0)))
    (`EquipmentBlueprintFn.SelectArmEquipmentByIndex` _asfgcharacter_player 3)))

(event `EnhancedInput|/EquipmentKeyBindings/Inputs/Player/Actions/IA_TriggerSelectEquipment_01`
  (params (ActionValue :type Boolean) (ElapsedSeconds :type "Float (double-precision)") (TriggeredSeconds :type "Float (double-precision)") (InputAction :type "InputAction Object Reference" :default "/EquipmentKeyBindings/Inputs/Player/Actions/IA_TriggerSelectEquipment_01.IA_TriggerSelectEquipment_01"))
  (:`Triggered`
    (bind _asfgcharacter_player (cast `FGCharacterPlayer` (`GameplayStatics.GetPlayerCharacter` 0)))
    (`EquipmentBlueprintFn.SelectArmEquipmentByIndex` _asfgcharacter_player)))

(event `self.ReceiveBeginPlay`
  (`self.EnableInput` (`GameplayStatics.GetPlayerController` 0)))

(event `EnhancedInput|/EquipmentKeyBindings/Inputs/Player/Actions/IA_TriggerSelectEquipment_02`
  (params (ActionValue :type Boolean) (ElapsedSeconds :type "Float (double-precision)") (TriggeredSeconds :type "Float (double-precision)") (InputAction :type "InputAction Object Reference" :default "/EquipmentKeyBindings/Inputs/Player/Actions/IA_TriggerSelectEquipment_02.IA_TriggerSelectEquipment_02"))
  (:`Triggered`
    (bind _asfgcharacter_player (cast `FGCharacterPlayer` (`GameplayStatics.GetPlayerCharacter` 0)))
    (`EquipmentBlueprintFn.SelectArmEquipmentByIndex` _asfgcharacter_player 1)))

(event `EnhancedInput|/EquipmentKeyBindings/Inputs/Player/Actions/IA_TriggerSelectEquipment_05`
  (params (ActionValue :type Boolean) (ElapsedSeconds :type "Float (double-precision)") (TriggeredSeconds :type "Float (double-precision)") (InputAction :type "InputAction Object Reference" :default "/EquipmentKeyBindings/Inputs/Player/Actions/IA_TriggerSelectEquipment_05.IA_TriggerSelectEquipment_05"))
  (:`Triggered`
    (bind _asfgcharacter_player (cast `FGCharacterPlayer` (`GameplayStatics.GetPlayerCharacter` 0)))
    (`EquipmentBlueprintFn.SelectArmEquipmentByIndex` _asfgcharacter_player 4)))

(event `EnhancedInput|/EquipmentKeyBindings/Inputs/Player/Actions/IA_TriggerSelectEquipment_06`
  (params (ActionValue :type Boolean) (ElapsedSeconds :type "Float (double-precision)") (TriggeredSeconds :type "Float (double-precision)") (InputAction :type "InputAction Object Reference" :default "/EquipmentKeyBindings/Inputs/Player/Actions/IA_TriggerSelectEquipment_06.IA_TriggerSelectEquipment_06"))
  (:`Triggered`
    (bind _asfgcharacter_player (cast `FGCharacterPlayer` (`GameplayStatics.GetPlayerCharacter` 0)))
    (`EquipmentBlueprintFn.SelectArmEquipmentByIndex` _asfgcharacter_player 5)))

(event `EnhancedInput|/EquipmentKeyBindings/Inputs/Player/Actions/IA_TriggerSelectEquipment_03`
  (params (ActionValue :type Boolean) (ElapsedSeconds :type "Float (double-precision)") (TriggeredSeconds :type "Float (double-precision)") (InputAction :type "InputAction Object Reference" :default "/EquipmentKeyBindings/Inputs/Player/Actions/IA_TriggerSelectEquipment_03.IA_TriggerSelectEquipment_03"))
  (:`Triggered`
    (bind _asfgcharacter_player (cast `FGCharacterPlayer` (`GameplayStatics.GetPlayerCharacter` 0)))
    (`EquipmentBlueprintFn.SelectArmEquipmentByIndex` _asfgcharacter_player 2)))

(fn `UserConstructionScript`)